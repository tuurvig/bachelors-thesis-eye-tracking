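; Player-controlled test subject for an eye-tracking heatmap setup, with movement and look input for both VR headset and desktop.
; On BeginPlay it configures the camera or tracking origin, spawns a HeatmapProducer and loads heatmaps from a hardcoded D: drive folder.
; Input toggles heatmaps, prints gaze-data status and sets a Painting flag.
; The heat-painting traces and timed export are disconnected, and Tick is empty.
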(event `self.ReceiveBeginPlay`
  (`|ExecutionSequence`
    (:`then_0`
      (if (`HeadMountedDisplayFunctionLibrary.IsHeadMountedDisplayEnabled`)
        (set `self.bUseControllerRotationYaw` false)
        (`HeadMountedDisplayFunctionLibrary.SetTrackingOrigin` "Floor")
        (else
          (`SceneComponent.K2_SetWorldLocation` (`self.Camera`) (0.0 0.0 170.0) false true))))
    (:`then_1`
      (bind _returnvalue (`|SpawnActorFromClass` "/EyeTrackingUtilities/Blueprints/HeatmapProducer.HeatmapProducer_C" (`KismetMathLibrary.MakeTransform` (0.0 0.0 0.0)) "AlwaysSpawn" "OverrideRootScale" self self))
      (set `self.EyeTrackingRuntime` _returnvalue))
    (:`then_2`
      (`/EyeTrackingUtilities/Blueprints/EyeTrackingHelperLibrary.LoadAllHeatmaps` "D:/Temp/Heatmaps/"))))

(event `InputAxis|MoveForward`
  (params (AxisValue :type "Float (single-precision)"))
  (`self.AddMovementInput` (select `bool` (`HeadMountedDisplayFunctionLibrary.IsHeadMountedDisplayEnabled`) :`false` (`self.GetActorForwardVector`) :`true` (`SceneComponent.GetForwardVector` (`self.Camera`))) AxisValue))

(event `InputAxis|MoveRight`
  (params (AxisValue :type "Float (single-precision)"))
  (`self.AddMovementInput` (select `bool` (`HeadMountedDisplayFunctionLibrary.IsHeadMountedDisplayEnabled`) :`false` (`self.GetActorRightVector`) :`true` (`SceneComponent.GetRightVector` (`self.Camera`))) AxisValue))

(event `InputAxis|Turn`
  (params (AxisValue :type "Float (single-precision)"))
  (`self.AddControllerYawInput` AxisValue))

(event `InputAxis|LookUp`
  (params (AxisValue :type "Float (single-precision)"))
  (`self.AddControllerPitchInput` AxisValue))

(event `InputAction|Fire`
  (params (Key :type "Key Structure"))
  (:`Pressed`
    (set `self.Painting` true))
  (:`Released`
    (set `self.Painting` false)))

(event `self.ReceiveTick`
  (params (DeltaSeconds :type "Float (single-precision)")))

(event `InputAction|EyeTrackingCalibration`
  (params (Key :type "Key Structure"))
  (:`Pressed`
    (bind (_outgazedata _returnvalue) (`EyeTrackerFunctionLibrary.GetGazeData`))
    (`KismetSystemLibrary.PrintString` (`KismetStringLibrary.Conv_BoolToString` _returnvalue))))

(event `ExportAllHeatmaps`
  (`/EyeTrackingUtilities/Blueprints/EyeTrackingHelperLibrary.ExportAllHeatmaps` "D:/Temp/Heatmaps"))

(event `InputAction|ToggleHeatmaps`
  (params (Key :type "Key Structure"))
  (:`Pressed`
    (`/EyeTrackingUtilities/Blueprints/EyeTrackingHelperLibrary.ToggleHeatmaps`)))

(fn `Incr`
  (`/Engine/EditorBlueprintResources/StandardMacros.IncrementInt` (`self.called`)))

(fn `UserConstructionScript`)