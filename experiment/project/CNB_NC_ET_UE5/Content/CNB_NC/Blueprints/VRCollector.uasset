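; VR pawn that records head and eye gaze heatmaps while the user moves through a scene.
; Movement input shifts the SceneOrigin actor opposite the camera's horizontal axes instead of moving the pawn.
; The EyeTrackingCalibration input starts a timed two-minute recording, then exports all heatmaps to disk.
; While recording, Tick emits frame-time-weighted rays through GazeEmitter along camera forward and, when confidence is sufficient, tracked eye gaze.
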(event `self.ReceiveBeginPlay`
  (`KismetSystemLibrary.ExecuteConsoleCommand` "stereo on" null)
  (set `self.bUseControllerRotationYaw` false)
  (`HeadMountedDisplayFunctionLibrary.SetTrackingOrigin` "Floor")
  (bind _returnvalue (`GameplayStatics.GetActorOfClass` "/Game/CNB_NC/Blueprints/SceneOrigin.SceneOrigin_C"))
  (set `self.SceneOrigin` _returnvalue))

(event `InputAxis|MoveForward`
  (params (AxisValue :type "Float (single-precision)"))
  (bind (_returnvalue_x _returnvalue_y) (`KismetMathLibrary.BreakVector` (`SceneComponent.GetForwardVector` (`self.Camera`))))
  (`self.K2_AddActorWorldOffset` (`self.SceneOrigin`) (* (* (`KismetMathLibrary.MakeVector` _returnvalue_x _returnvalue_y) -2.0) AxisValue) false true))

(event `InputAxis|MoveRight`
  (params (AxisValue :type "Float (single-precision)"))
  (bind (_returnvalue_x _returnvalue_y) (`KismetMathLibrary.BreakVector` (`SceneComponent.GetRightVector` (`self.Camera`))))
  (`self.K2_AddActorWorldOffset` (`self.SceneOrigin`) (* (* (`KismetMathLibrary.MakeVector` _returnvalue_x _returnvalue_y) -2.0) AxisValue) false true))

(event `InputAction|ToggleHeatmaps`
  (params (Key :type "Key Structure"))
  (:`Pressed`
    (`/EyeTrackingUtilities/Blueprints/EyeTrackingHelperLibrary.ToggleHeatmaps`)))

(event `self.ReceiveTick`
  (params (DeltaSeconds :type "Float (single-precision)"))
  (bind _camera (`self.Camera`))
  (if (`self.Start`)
    (`/EyeTrackingUtilities/Blueprints/GazeEmitter.EmitRayFrom` (`self.GazeEmitter`) (`SceneComponent.K2_GetComponentLocation` _camera) (`SceneComponent.GetForwardVector` _camera) "NewEnumerator1" DeltaSeconds)
    (bind _outgazedata (`EyeTrackerFunctionLibrary.GetGazeData`))
    (if (> (`.ConfidenceValue` (break `EyeTrackerGazeData` _outgazedata)) 0.5)
      (`/EyeTrackingUtilities/Blueprints/GazeEmitter.EmitRayFrom` (`self.GazeEmitter`) (break `EyeTrackerGazeData` _outgazedata) (`.GazeDirection` (break `EyeTrackerGazeData` _outgazedata)) "NewEnumerator0" DeltaSeconds))))

(event `InputAction|EyeTrackingCalibration`
  (params (Key :type "Key Structure"))
  (:`Pressed`
    (set `self.Start` true)
    (`KismetSystemLibrary.Delay` 120.0)
    (`/EyeTrackingUtilities/Blueprints/EyeTrackingHelperLibrary.ExportAllHeatmaps` "C:/ProgramData/NC_ET/")
    (set `self.Start` false)))

(fn `UserConstructionScript`)