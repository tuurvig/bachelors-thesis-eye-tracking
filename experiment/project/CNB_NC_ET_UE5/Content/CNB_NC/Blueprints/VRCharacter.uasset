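; VRCharacter is a VR character Blueprint that drives its camera and body from headset tracking every tick.
; CameraTransform applies only device pitch and roll to the camera, when the headset is enabled.
; CapsuleTransform sets actor yaw from the device and teleports it by a local offset computed from device position, camera relative location and actor location.
; The initial rotation saved at BeginPlay feeds only an unused yaw sum.
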(event `self.ReceiveBeginPlay`
  (set `self.InitialWorldRotation` (`self.K2_GetActorRotation`)))

(event `self.ReceiveTick`
  (params (DeltaSeconds :type "Float (single-precision)"))
  (`self.CameraTransform`)
  (`self.CapsuleTransform`))

(fn `CameraTransform`
  (bind _devicerotation (`HeadMountedDisplayFunctionLibrary.GetOrientationAndPosition`))
  (if (`HeadMountedDisplayFunctionLibrary.IsHeadMountedDisplayEnabled`)
    (`SceneComponent.K2_SetRelativeRotation` (`self.Camera`) (`KismetMathLibrary.MakeRotator` (.roll _devicerotation) (.pitch _devicerotation)) false true)))

(fn `CapsuleTransform`
  (bind (_devicerotation _deviceposition) (`HeadMountedDisplayFunctionLibrary.GetOrientationAndPosition`))
  (`self.K2_SetActorRotation` (`KismetMathLibrary.MakeRotator` 0.0 0.0 (.yaw _devicerotation)) true)
  (`self.K2_AddActorLocalOffset` (- (- _deviceposition (`SceneComponent.RelativeLocation` (`self.Camera`))) (`self.K2_GetActorLocation`)) false true))

(fn `UserConstructionScript`)