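; ETCharacter is a character Blueprint that serves as a debug readout for eye-tracking gaze data.
; Every Tick calls the parent, polls GetGazeData, then prints its return value and the gaze direction through PrintString.
; The gaze data drives nothing else, BeginPlay is a disabled placeholder, and the construction script only calls the parent.
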(event `self.ReceiveTick`
  (params (DeltaSeconds :type "Float (single-precision)"))
  (`parent.ReceiveTick` DeltaSeconds)
  (bind (_outgazedata _returnvalue) (`EyeTrackerFunctionLibrary.GetGazeData`))
  (`KismetSystemLibrary.PrintString` (`KismetStringLibrary.Conv_BoolToString` _returnvalue))
  (`KismetSystemLibrary.PrintString` (`KismetStringLibrary.Conv_VectorToString` (`.GazeDirection` (break `EyeTrackerGazeData` _outgazedata)))))

(event `InputAction|EyeTrackingCalibration`
  (params (Key :type "Key Structure")))

(fn `UserConstructionScript`
  (`parent.UserConstructionScript`))