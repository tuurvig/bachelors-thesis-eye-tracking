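; SceneObserver is a player pawn for walking through a scene and viewing heatmap visualisations.
; On BeginPlay it teleports its camera to a fixed world position at standing height and loads all heatmaps from a hard-coded local ProgramData folder.
; Axis inputs drive movement and look, while the ToggleHeatmaps action cycles heatmap materials.
; The heatmap load and toggle functions are called here but defined outside this graph.
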(event `self.ReceiveBeginPlay`
  ;[1 1 1] Set height of the pawn in the scene and load all heatmaps
  (`SceneComponent.K2_SetWorldLocation` (`self.Camera`) (0.0 0.0 170.0) false true)
  (`/EyeTrackingUtilities/Blueprints/EyeTrackingHelperLibrary.LoadAllHeatmaps` "C:/ProgramData/NC_ET/"))

(event `InputAxis|MoveForward`
  (params (AxisValue :type "Float (single-precision)"))
  ;[1 1 1] Scene traversal logic using inputs
  (`self.AddMovementInput` (`self.GetActorForwardVector`) AxisValue))

(event `InputAxis|Turn`
  (params (AxisValue :type "Float (single-precision)"))
  ;[1 1 1] Scene traversal logic using inputs
  (`self.AddControllerYawInput` AxisValue))

(event `InputAxis|MoveRight`
  (params (AxisValue :type "Float (single-precision)"))
  ;[1 1 1] Scene traversal logic using inputs
  (`self.AddMovementInput` (`self.GetActorRightVector`) AxisValue))

(event `InputAxis|LookUp`
  (params (AxisValue :type "Float (single-precision)"))
  ;[1 1 1] Scene traversal logic using inputs
  (`self.AddControllerPitchInput` AxisValue))

(event `InputAction|ToggleHeatmaps`
  (params (Key :type "Key Structure"))
  ;[1 1 1] Cycle through heatmap visualisation materials
  (:`Pressed`
    (`/EyeTrackingUtilities/Blueprints/EyeTrackingHelperLibrary.ToggleHeatmaps`)))

(fn `UserConstructionScript`)