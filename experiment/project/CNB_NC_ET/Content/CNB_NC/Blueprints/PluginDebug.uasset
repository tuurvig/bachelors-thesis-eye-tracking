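; PluginDebug is a first-person debug pawn for testing gaze heatmap painting and visualisation.
; It sets the camera height at start, handles move and look axes, and cycles heatmap materials on ToggleHeatmaps.
; While Fire is held, Tick casts two GazeEmitter rays of different types along the camera's view, with strength scaled by frame time.
; The LoadAllHeatmaps call is disconnected, so saved heatmaps never load despite the BeginPlay comment.
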(event `self.ReceiveBeginPlay`
  ;[1 1 1] Set height of the pawn in the scene and load all heatmaps
  (`SceneComponent.K2_SetWorldLocation` (`self.Camera`) (0.0 0.0 170.0) false true))

(event `InputAxis|MoveForward`
  (params (AxisValue :type "Float (single-precision)"))
  ;[1 1 1] Scene traversal logic using inputs
  (`self.AddMovementInput` (`self.GetActorForwardVector`) AxisValue))

(event `InputAxis|Turn`
  (params (AxisValue :type "Float (single-precision)"))
  ;[1 1 1] Scene traversal logic using inputs
  (`self.AddControllerYawInput` AxisValue))

(event `InputAxis|MoveRight`
  (params (AxisValue :type "Float (single-precision)"))
  ;[1 1 1] Scene traversal logic using inputs
  (`self.AddMovementInput` (`self.GetActorRightVector`) AxisValue))

(event `InputAxis|LookUp`
  (params (AxisValue :type "Float (single-precision)"))
  ;[1 1 1] Scene traversal logic using inputs
  (`self.AddControllerPitchInput` AxisValue))

(event `InputAction|ToggleHeatmaps`
  (params (Key :type "Key Structure"))
  ;[1 1 1] Cycle through heatmap visualisation materials
  (:`Pressed`
    (`/EyeTrackingUtilities/Blueprints/EyeTrackingHelperLibrary.ToggleHeatmaps`)))

(event `InputAction|Fire`
  (params (Key :type "Key Structure"))
  (:`Pressed`
    (set `self.Painting` true))
  (:`Released`
    (set `self.Painting` false)))

(event `self.ReceiveTick`
  (params (DeltaSeconds :type "Float (single-precision)"))
  (bind _camera (`self.Camera`))
  (bind _returnvalue (`SceneComponent.K2_GetComponentLocation` _camera))
  (bind _returnvalue_2 (`SceneComponent.GetForwardVector` _camera))
  ;[1 1 1] Heatmap rendering cycle
  (if (`self.Painting`)
    (`/EyeTrackingUtilities/Blueprints/GazeEmitter.EmitRayFrom` (`self.GazeEmitter`) _returnvalue _returnvalue_2 "NewEnumerator1" DeltaSeconds)
    (`/EyeTrackingUtilities/Blueprints/GazeEmitter.EmitRayFrom` (`self.GazeEmitter`) _returnvalue _returnvalue_2 "NewEnumerator0" DeltaSeconds)))

(fn `UserConstructionScript`)