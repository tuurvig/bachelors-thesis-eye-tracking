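; VRCollector is a VR pawn that records gaze heatmaps during a timed experiment.
; Movement input shifts a SceneOrigin actor opposite to the camera's flattened forward and right vectors, imitating traversal by moving the scene instead of the pawn.
; While the experiment runs, each tick emits two rays along the camera's forward vector through GazeEmitter, weighted by frame time.
; After three minutes it exports all heatmaps to disk and quits; a separate input toggles heatmaps.
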(event `self.ReceiveBeginPlay`
  ;[1 1 1] Initialise the pawn
  (`KismetSystemLibrary.ExecuteConsoleCommand` "xhmd" null)
  (set `self.bUseControllerRotationYaw` false)
  (`HeadMountedDisplayFunctionLibrary.SetTrackingOrigin` "Floor")
  (bind _returnvalue (`GameplayStatics.GetActorOfClass` "/Game/CNB_NC/Blueprints/SceneOrigin.SceneOrigin_C"))
  (set `self.SceneOrigin` _returnvalue))

(event `InputAxis|MoveForward`
  (params (AxisValue :type "Float (single-precision)"))
  (bind (_returnvalue_x _returnvalue_y) (`KismetMathLibrary.BreakVector` (`SceneComponent.GetForwardVector` (`self.Camera`))))
  ;[1 1 1] Move with pseudo scene origin to imitate scene traversal
  (`self.K2_AddActorWorldOffset` (`self.SceneOrigin`) (* (* (`KismetMathLibrary.MakeVector` _returnvalue_x _returnvalue_y) -5.0) AxisValue) false true))

(event `InputAxis|MoveRight`
  (params (AxisValue :type "Float (single-precision)"))
  (bind (_returnvalue_x _returnvalue_y) (`KismetMathLibrary.BreakVector` (`SceneComponent.GetRightVector` (`self.Camera`))))
  ;[1 1 1] Move with pseudo scene origin to imitate scene traversal
  (`self.K2_AddActorWorldOffset` (`self.SceneOrigin`) (* (* (`KismetMathLibrary.MakeVector` _returnvalue_x _returnvalue_y) -5.0) AxisValue) false true))

(event `InputAction|ToggleHeatmaps`
  (params (Key :type "Key Structure"))
  (:`Pressed`
    (`/EyeTrackingUtilities/Blueprints/EyeTrackingHelperLibrary.ToggleHeatmaps`)))

(event `self.ReceiveTick`
  (params (DeltaSeconds :type "Float (single-precision)"))
  (bind _camera (`self.Camera`))
  (bind _returnvalue (`SceneComponent.K2_GetComponentLocation` _camera))
  (bind _returnvalue_2 (`SceneComponent.GetForwardVector` _camera))
  ;[1 1 1] Heatmap rendering cycle
  (if (`self.Start`)
    (`/EyeTrackingUtilities/Blueprints/GazeEmitter.EmitRayFrom` (`self.GazeEmitter`) _returnvalue _returnvalue_2 "NewEnumerator1" DeltaSeconds)
    (`/EyeTrackingUtilities/Blueprints/GazeEmitter.EmitRayFrom` (`self.GazeEmitter`) _returnvalue _returnvalue_2 "NewEnumerator0" DeltaSeconds)))

(event `InputAction|StartExperiment`
  (params (Key :type "Key Structure"))
  ;[1 1 1] Start the experiment for a defined time and export heatmaps when it ends.
  (:`Pressed`
    (if (not (`self.Start`))
      (set `self.Start` true)
      (`KismetSystemLibrary.Delay` 180.0)
      (`/EyeTrackingUtilities/Blueprints/EyeTrackingHelperLibrary.ExportAllHeatmaps` "C:/ProgramData/NC_ET/")
      (set `self.Start` false)
      (`KismetSystemLibrary.QuitGame` null "Quit"))))

(fn `UserConstructionScript`)