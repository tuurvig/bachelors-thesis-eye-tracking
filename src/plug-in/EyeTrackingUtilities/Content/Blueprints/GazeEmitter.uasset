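; GazeEmitter casts gaze rays into the world to paint heat onto eye-tracked static meshes.
; On BeginPlay it spawns and stores a HeatmapProducer.
; EmitRayFrom traces static and dynamic objects, keeping only hits on EyeTrackedStaticMeshComponents, then re-traces that single component for a complex hit.
; That hit's location, normal and distance go to the HeatmapProducer along with direction, ray type and doubled strength.
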(event `self.ReceiveBeginPlay`
  ;[1 1 1] Spawn HeatmapProducer in the scene and save it as a variable
  (bind _returnvalue (`|SpawnActorFromClass` "/EyeTrackingUtilities/Blueprints/HeatmapProducer.HeatmapProducer_C" (`KismetMathLibrary.MakeTransform` (0.0 0.0 0.0)) "AlwaysSpawn" "OverrideRootScale" null null))
  (set `self.HeatmapProducer` _returnvalue))

(fn `EmitRayFrom`
  (params (Origin :type "Vector Structure") (Direction :type "Vector Structure") (RayType :type "/EyeTrackingUtilities/Blueprints/HeatType Enum" :default "NewEnumerator0") (Strength :type "Float (double-precision)"))
  ;[1 1 1] Acquire complex world hit from origin and direction.
  (bind (_hit_ _hit _eyetracked_component) (`self.Get World Hit from Gaze` Origin Direction 20000.0))
  (if _hit_
    (bind (_outcomponent _outhit) (`self.GetComplexFromSimpleHit` _hit _eyetracked_component))
    (bind (_bblockinghit _binitialoverlap _time _distance _location _impactpoint _normal) (`GameplayStatics.BreakHitResult` _outhit))
    (`/EyeTrackingUtilities/Blueprints/HeatmapProducer.ApplyHeatToComponent` (`self.HeatmapProducer`) _outcomponent _location (`local.Direction`) _normal _distance (* (`local.Strength`) 2.0) (`local.RayType`))))

(fn `Get World Hit from Gaze`
  (params (GazeOrigin :type "Vector Structure") (GazeDirection :type "Vector Structure") (Distance :type "Float (double-precision)"))
  (returns (`Hit?` :type Boolean) (Hit :type "HitResult Structure") (`EyeTracked Component` :type "/EyeTrackingUtilities/Blueprints/EyeTrackedStaticMeshComponent Object Reference"))
  ;[1 1 1] Send trace for all static and dynamic objects
  (bind (_outhit _returnvalue) (`KismetSystemLibrary.LineTraceSingleForObjects` GazeOrigin (+ GazeOrigin (* GazeDirection Distance)) (`|MakeArray` "ObjectTypeQuery1" "ObjectTypeQuery2" :!type "EObjectTypeQuery Enum")))
  ;[1 1 1] Return hit only when it is a successful hit on a EyeTrackedStaticMesh
  (if _returnvalue
    (bind _aseye_tracked_static_mesh_component (cast `/EyeTrackingUtilities/Blueprints/EyeTrackedStaticMeshComponent` (`.HitComponent` (`GameplayStatics.BreakHitResult` _outhit)))
      (:`then`
        (return true _outhit _aseye_tracked_static_mesh_component))
      (:`CastFailed`
        _)))
  (return false (struct) null))

(fn `GetComplexFromSimpleHit`
  (params (IncomingHit :type "HitResult Structure") (EyeTrackedComponent :type "/EyeTrackingUtilities/Blueprints/EyeTrackedStaticMeshComponent Object Reference"))
  (returns (outComponent :type "/EyeTrackingUtilities/Blueprints/EyeTrackedStaticMeshComponent Object Reference") (outHit :type "HitResult Structure"))
  (bind (_bblockinghit _binitialoverlap _time _distance _location _impactpoint _normal _impactnormal _physmat _hitactor _hitcomponent _hitbonename _hititem _elementindex _faceindex _tracestart _traceend) (`GameplayStatics.BreakHitResult` IncomingHit))
  ;[1 1 1] Send a trace again to a get a complex hit on a single component
  (bind (_hitlocation _hitnormal _bonename _outhit) (`PrimitiveComponent.K2_LineTraceComponent` EyeTrackedComponent _tracestart _traceend true false false))
  (return EyeTrackedComponent _outhit))