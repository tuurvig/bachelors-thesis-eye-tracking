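; Actor that paints gaze or camera heat splats onto eye-tracked components by rendering them into heatmap textures.
; It sizes and places an orthographic scene capture and background plane to the target resolution, limiting the capture to the component and plane.
; It temporarily swaps in a dynamic UV-unwrap brush material fed with hit data and distance-scaled radius, captures, then restores the original material.
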(fn `AlignRenderer`
  (params (Resolution :type Integer) (Location :type "Vector Structure"))
  (locals (SceneCaptureShift :type "Vector Structure" :default (0.0 0.0 10.0)) (RenderPlaneShift :type "Vector Structure" :default (0.0 0.0 -1.0)))
  (bind _returnvalue (`KismetMathLibrary.Conv_IntToDouble` Resolution))
  (bind _unwrapuvcapture (`self.UnwrapUVCapture`))
  (bind _renderplane (`self.RenderPlane`))
  (bind _unwrapmaterial (`self.UnwrapMaterial`))
  (bind _returnvalue_2 (* _returnvalue 0.01))
  ;[1 1 1] Align background plane and scene capture to be of size of the texture they are about to render to.
  (`|ExecutionSequence`
    (:`then_0`
      (bind _output_get (set `SceneCaptureComponent2D.OrthoWidth` _returnvalue _unwrapuvcapture))
      (`SceneComponent.SetWorldScale3D` _renderplane (`KismetMathLibrary.MakeVector` _returnvalue_2 _returnvalue_2))
      (`MaterialInstanceDynamic.SetScalarParameterValue` _unwrapmaterial "CaptureSize" _output_get))
    (:`then_1`
      (`SceneComponent.K2_SetWorldLocation` _unwrapuvcapture (+ Location (`local.SceneCaptureShift`)) false true)
      (`SceneComponent.K2_SetWorldLocation` _renderplane (+ Location (`local.RenderPlaneShift`)) false true)
      (`MaterialInstanceDynamic.SetVectorParameterValue` _unwrapmaterial "UnwrapLocation" (`KismetMathLibrary.Conv_VectorToLinearColor` (`local.Location`))))))

(fn `ApplyHeatToComponent`
  (params (EyeTrackedComponent :type "/EyeTrackingUtilities/Blueprints/EyeTrackedStaticMeshComponent Object Reference") (HitLocation :type "Vector Structure") (HitDirection :type "Vector Structure") (HitNormal :type "Vector Structure") (Distance :type "Float (double-precision)") (Strength :type "Float (double-precision)") (HeatType :type "/EyeTrackingUtilities/Blueprints/HeatType Enum" :default "NewEnumerator0"))
  ;[1 1 1] Prepares the Actor to unwrap and render the input ET component.
  (`|ExecutionSequence`
    (:`then_0`
      (`self.ShowRenderPlane`)
      (`self.AlignRenderer` (select `/EyeTrackingUtilities/Blueprints/HeatType` HeatType :`NewEnumerator0` (`/EyeTrackingUtilities/Blueprints/EyeTrackedStaticMeshComponent.GazeResolution` EyeTrackedComponent) :`NewEnumerator1` (`/EyeTrackingUtilities/Blueprints/EyeTrackedStaticMeshComponent.CameraResolution` EyeTrackedComponent)) (`SceneComponent.K2_GetComponentLocation` EyeTrackedComponent)))
    (:`then_1`
      (`self.PrepareScene` EyeTrackedComponent))
    (:`then_2`
      (`self.RenderSplatOntoComponent` EyeTrackedComponent HitLocation HitDirection HitNormal Distance Strength HeatType)
      (`self.HideRenderPlane`))))

(fn `HideRenderPlane`
  (`SceneComponent.SetVisibility` (`self.RenderPlane`) false false))

(fn `MakeRadiusFromDistance`
  (params (Distance :type "Float (double-precision)") (Type :type "/EyeTrackingUtilities/Blueprints/HeatType Enum" :default "NewEnumerator0"))
  (returns (Radius :type "Float (double-precision)"))
  (return (* Distance (select `/EyeTrackingUtilities/Blueprints/HeatType` Type :`NewEnumerator0` 0.05 :`NewEnumerator1` 0.5))))

(fn `PrepareScene`
  (params (EyeTrackedComponent :type "/EyeTrackingUtilities/Blueprints/EyeTrackedStaticMeshComponent Object Reference"))
  (bind _unwrapuvcapture (`self.UnwrapUVCapture`))
  ;[1 1 1] Define only those objects that will be part of the heatmap render.
  (`SceneCaptureComponent.ClearShowOnlyComponents` _unwrapuvcapture)
  (`SceneCaptureComponent.ShowOnlyComponent` _unwrapuvcapture EyeTrackedComponent)
  (`SceneCaptureComponent.ShowOnlyComponent` _unwrapuvcapture (`self.RenderPlane`)))

(fn `RenderSplatOntoComponent`
  (params (EyeTrackedComponent :type "/EyeTrackingUtilities/Blueprints/EyeTrackedStaticMeshComponent Object Reference") (Location :type "Vector Structure") (Direction :type "Vector Structure") (Normal :type "Vector Structure") (Distance :type "Float (double-precision)") (Strength :type "Float (double-precision)") (HeatType :type "/EyeTrackingUtilities/Blueprints/HeatType Enum" :default "NewEnumerator0"))
  (locals (OriginalMaterial :type "MaterialInterface Object Reference"))
  (bind _unwrapmaterial (`self.UnwrapMaterial`))
  (bind _eyetrackedcomponent (`local.EyeTrackedComponent`))
  (bind _unwrapuvcapture (`self.UnwrapUVCapture`))
  ;[1 1 1] Save the original material to local variable
  (set `local.OriginalMaterial` (`PrimitiveComponent.GetMaterial` EyeTrackedComponent 0))
  (`|ExecutionSequence`
    (:`then_0`
      ;[1 1 1] Set all material parameters of UnwrapMaterial dynamic material instance
      (`MaterialInstanceDynamic.SetVectorParameterValue` _unwrapmaterial "HitLocation" (`KismetMathLibrary.Conv_VectorToLinearColor` (`local.Location`)))
      (`MaterialInstanceDynamic.SetVectorParameterValue` _unwrapmaterial "DirectionToCamera" (`KismetMathLibrary.Conv_VectorToLinearColor` (* (`local.Direction`) -1.0)))
      (`MaterialInstanceDynamic.SetVectorParameterValue` _unwrapmaterial "HitNormal" (`KismetMathLibrary.Conv_VectorToLinearColor` (`local.Normal`)))
      (`MaterialInstanceDynamic.SetScalarParameterValue` _unwrapmaterial "BrushRadius" (`self.MakeRadiusFromDistance` (`local.Distance`) (`local.HeatType`)))
      (`MaterialInstanceDynamic.SetScalarParameterValue` _unwrapmaterial "Strength" (`local.Strength`)))
    (:`then_1`
      ;[1 1 1] Set the unwrap material to Primitive's main material slot and assign to the capture component a texture to which it will be rendered.
      (`/EyeTrackingUtilities/Blueprints/EyeTrackedStaticMeshComponent.AttachRenderer` _eyetrackedcomponent _unwrapuvcapture (`local.HeatType`))
      (`PrimitiveComponent.SetMaterial` _eyetrackedcomponent 0 (`self.UnwrapMaterial`)))
    (:`then_2`
      ;[1 1 1] Capture the unwrapped mesh and set its material back to its original one.
      (`SceneCaptureComponent2D.CaptureScene` _unwrapuvcapture)
      (`PrimitiveComponent.SetMaterial` _eyetrackedcomponent 0 (`local.OriginalMaterial`)))))

(fn `ShowRenderPlane`
  (`SceneComponent.SetVisibility` (`self.RenderPlane`) true false))

(fn `UserConstructionScript`
  ;[1 1 1] Initialise the dynamic UnwrapBrush material
  (bind _returnvalue (`KismetMaterialLibrary.CreateDynamicMaterialInstance` "/EyeTrackingUtilities/Materials/UnwrapBrush.UnwrapBrush"))
  (set `self.UnwrapMaterial` _returnvalue))